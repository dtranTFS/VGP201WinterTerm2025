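; Health component for the FPS game that stores an actor's health and offers healing, damage, full heal, kill, death check and normalized-health functions.
; BeginPlay runs Init with the configured min and max, which starts health at the maximum.
; Heal and Damage reject non-positive amounts with a printed message, then route through SetHealth, which clamps to the min/max range.
; No events are broadcast on change or death.
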(event `self.ReceiveBeginPlay`
  (`self.Init` (`self.MinHealth`) (`self.MaxHealth`)))

(fn `ClampHealth`
  (params (Value :type "Float (double-precision)"))
  (returns (`Return Value` :type "Float (double-precision)"))
  (return (`KismetMathLibrary.FClamp` Value (`self.MinHealth`) (`self.MaxHealth`))))

(fn `Damage`
  (params (`Damage Amt` :type "Float (double-precision)"))
  (if (> `Damage Amt` 0.0)
    (`self.SetHealth` (- (`self.GetHealth`) `Damage Amt`))
    (else
      (`KismetSystemLibrary.PrintString` "Damage value must be positive!"))))

(fn `GetHealth`
  (returns (Health :type "Float (double-precision)"))
  (return (`self.Health`)))

(fn `GetNormalizedHealth`
  (returns (Value :type "Float (double-precision)"))
  (return (`KismetMathLibrary.FClamp` (/ (`self.GetHealth`) (`self.MaxHealth`)))))

(fn `Heal`
  (params (`Heal Amt` :type "Float (double-precision)"))
  (if (> `Heal Amt` 0.0)
    (`self.SetHealth` (+ (`self.GetHealth`) `Heal Amt`))
    (else
      (`KismetSystemLibrary.PrintString` "Heal value must be positive!"))))

(fn `HealFull`
  (`self.Heal` (`self.MaxHealth`)))

(fn `Init`
  (params (`New Min Health` :type "Float (double-precision)") (`New Max Health` :type "Float (double-precision)"))
  (set `self.MinHealth` `New Min Health`)
  (bind _output_get (set `self.MaxHealth` `New Max Health`))
  (`self.SetHealth` _output_get))

(fn `IsDead`
  (returns (Value :type Boolean))
  (return (<= (`self.GetHealth`) (`self.MinHealth`))))

(fn `Kill`
  (`self.Damage` (`self.MaxHealth`)))

(fn `SetHealth`
  (params (`New Health` :type "Float (double-precision)"))
  (returns (Health :type "Float (double-precision)"))
  (bind _output_get (set `self.Health` (`self.ClampHealth` `New Health`)))
  (return _output_get))