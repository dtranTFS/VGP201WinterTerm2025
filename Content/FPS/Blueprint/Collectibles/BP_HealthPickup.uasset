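; BP_HealthPickup is a collectible that heals the player by HealAmount when collected.
; It overrides OnCollect, runs the parent logic, then casts player character 0 to BP_FPSCharacter and calls its Heal function.
; Disconnected leftover nodes show an older approach that healed the health component directly and updated the game menu's health bar through the game mode.
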(fn `OnCollect`
  (`parent.OnCollect`)
  (bind _asbp_fpscharacter (cast `/Game/FPS/Blueprint/Player/BP_FPSCharacter` (`GameplayStatics.GetPlayerCharacter` 0)))
  (`/Game/FPS/Blueprint/Player/BP_FPSCharacter.Heal` _asbp_fpscharacter (`self.HealAmount`)))

(fn `UserConstructionScript`
  (`parent.UserConstructionScript`))